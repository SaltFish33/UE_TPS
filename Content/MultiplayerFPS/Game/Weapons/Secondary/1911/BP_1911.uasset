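; BP_1911 is the 1911 secondary weapon Blueprint for the multiplayer FPS, with its only active custom logic toggling magazine visibility.
; ToggleMagazineVisibility swaps material slot 1 on the first- and third-person meshes between the 1911 material and an invisible one.
; Hiding applies to both meshes immediately, while showing updates the first-person mesh first and the third-person mesh after a short delay.
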(event EventBeginPlay
  (|CallParentFunction) ; This node is disabled and will not be called.\nDrag off pins to build functionality.
)

(event Collision|EventActorBeginOverlap
  (params (OtherActor :type Actor%20Object%20Reference)))

(event EventTick
  (params (DeltaSeconds :type Float%20%28single-precision%29))
  (|CallParentFunction DeltaSeconds) ; This node is disabled and will not be called.\nDrag off pins to build functionality.
)

(event EventToggleMagazineVisibility
  (params (Visibility :type Boolean))
  (if Visibility
    (Rendering|Material|SetMaterial (Variables|Default|GetFPMesh) 1 "/Game/MultiplayerFPS/Game/Weapons/Secondary/1911/Mesh/Materials/M_1911.M_1911")
    (Utilities|FlowControl|Delay 0.1)
    (Rendering|Material|SetMaterial (Variables|Default|GetTPMesh) 1 "/Game/MultiplayerFPS/Game/Weapons/Secondary/1911/Mesh/Materials/M_1911.M_1911")
    (else
      (Rendering|Material|SetMaterial (Variables|Default|GetFPMesh) 1 "/Game/MultiplayerFPS/Game/Effects/M_Invisible.M_Invisible"))))

(fn ConstructionScript
  (|CallParentFunction))