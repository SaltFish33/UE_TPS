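; Karambit knife melee weapon for the multiplayer FPS that varies its swipe animations.
; A looping half-second timer starts on BeginPlay and steps a counter through four montage choices, independently of attack input.
; Each step sets the first-person fire montage and third-person weapon fire montage from left and right swing variants.
; Hit and miss variants come from the same cycle, with no hit check in this Blueprint.
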(event Custom|SelectSlashAnim
  (bind _result (Math|Integer|IncrementInt (Variables|Default|GetInt))
    (:%20%20
      (if (> _result 3)
        (Variables|Default|SetInt 0))
      (Variables|Default|SetFPMontage_Fire (Utilities|Select :Index (Variables|Default|GetInt) :Option%200 "/Game/MultiplayerFPS/Game/Weapons/Melee/Karambit/Animations/FirstPersonAnimations/c_karambit_left_swipe_hit_Montage.c_karambit_left_swipe_hit_Montage" :Option%201 "/Game/MultiplayerFPS/Game/Weapons/Melee/Karambit/Animations/FirstPersonAnimations/c_karambit_left_swipe_miss_Montage.c_karambit_left_swipe_miss_Montage" :Option%202 "/Game/MultiplayerFPS/Game/Weapons/Melee/Karambit/Animations/FirstPersonAnimations/c_karambit_right_swipe_hit_Montage.c_karambit_right_swipe_hit_Montage" :Option%203 "/Game/MultiplayerFPS/Game/Weapons/Melee/Karambit/Animations/FirstPersonAnimations/c_karambit_right_swipe_miss_Montage.c_karambit_right_swipe_miss_Montage"))
      (Variables|Default|SetTPMontage_FireWeapon (Utilities|Select :Index (Variables|Default|GetInt) :Option%200 "/Game/MultiplayerFPS/Game/Weapons/Melee/Karambit/Animations/ThirdPersonAnimations/c_3p_karambit_swing_left_hit_Montage.c_3p_karambit_swing_left_hit_Montage" :Option%201 "/Game/MultiplayerFPS/Game/Weapons/Melee/Karambit/Animations/ThirdPersonAnimations/c_3p_karambit_swing_left_miss_Montage.c_3p_karambit_swing_left_miss_Montage" :Option%202 "/Game/MultiplayerFPS/Game/Weapons/Melee/Karambit/Animations/ThirdPersonAnimations/c_3p_karambit_swing_right_hit1_Montage.c_3p_karambit_swing_right_hit1_Montage" :Option%203 "/Game/MultiplayerFPS/Game/Weapons/Melee/Karambit/Animations/ThirdPersonAnimations/c_3p_karambit_swing_right_hit_Montage.c_3p_karambit_swing_right_hit_Montage")))))

(event EventBeginPlay
  (|CallParentFunction)
  (Utilities|Time|SetTimerbyEvent (delegate Custom|SelectSlashAnim) 0.5 true))

(event Collision|EventActorBeginOverlap
  (params (OtherActor :type Actor%20Object%20Reference)))

(event EventTick
  (params (DeltaSeconds :type Float%20%28single-precision%29)))

(fn ConstructionScript
  (|CallParentFunction))