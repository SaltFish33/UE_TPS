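; Pistol flashlight attachment for a multiplayer FPS, with a mesh and spotlight configured separately for first-person and third-person copies.
; On BeginPlay it runs a visibility event: the FP copy becomes owner-only and shadowless, while the TP copy hides from its owner and switches off its spotlight.
; UpdateVisibility flips each copy's owner visibility when the view mode changes.
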(event Custom|MC_Visibility
  ;[1 1 1] Set FP and TP parts Visiblity
  (if (Variables|Default|GetVisibility)
    (if (Variables|Default|GetFP?)
      (Rendering|SetOnlyOwnerSee (Variables|Default|GetMesh) true :!class /Script/Engine.PrimitiveComponent)
      (Rendering|SetCastShadow (Variables|Default|GetMesh) false)
      (elif (Variables|Default|GetTP?)
        (Class|PrimitiveComponent|SetOwnerNoSee (Variables|Default|GetMesh) true)
        (Rendering|SetVisibility (Variables|Default|GetSpotLight) false false)
        (Components|Activation|SetAutoActivate (Variables|Default|GetSpotLight) false)))))

(event EventBeginPlay
  (|CallParentFunction)
  (CallFunction|MCVisibility))

(event EventTick
  (params (DeltaSeconds :type Float%20%28single-precision%29))
  (|CallParentFunction DeltaSeconds))

(event EventUpdateVisibility
  (params (NewViewMode :type Boolean))
  (if (Variables|Default|GetFP?)
    (Class|PrimitiveComponent|SetOwnerNoSee (Variables|Default|GetMesh) NewViewMode)
    (else
      (Class|PrimitiveComponent|SetOwnerNoSee (Variables|Default|GetMesh) (not NewViewMode)))))

(event Collision|EventActorBeginOverlap
  (params (OtherActor :type Actor%20Object%20Reference))
  (|CallParentFunction OtherActor) ; This node is disabled and will not be called.\nDrag off pins to build functionality.
)

(fn ConstructionScript
  (|CallParentFunction))