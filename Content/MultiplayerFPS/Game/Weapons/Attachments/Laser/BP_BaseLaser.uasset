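; Base laser sight attachment for weapons, showing a beam and a dot that can toggle on/off and switch to an infrared mode.
; At BeginPlay it configures owner visibility and shadows for first- and third-person copies, with view-mode changes updating visibility.
; On Tick, non-third-person copies trace forward while toggled on, stretching the beam to the hit and aligning the dot to the surface.
; Infrared mode swaps the beam material and widens the beam.
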(event Custom|MC_Visibility
  ;[1 1 1] Set FP and TP parts Visiblity
  (if (Variables|Default|GetVisibility)
    (if (Variables|Default|GetFP?)
      (Rendering|SetOnlyOwnerSee (Variables|Default|GetStaticMesh) true :!class /Script/Engine.PrimitiveComponent)
      (Rendering|SetCastShadow (Variables|Default|GetStaticMesh) false)
      (bind _asbp_weapon_base (Utilities|Casting|CastToBP_WeaponBase (Components|GetOwner)))
      (bind _playerref (Variables|/Game/MultiplayerFPS/Game/Blueprints/Core/BP_WeaponBase.BP_WeaponBase_C|GetPlayerRef _asbp_weapon_base)
        (:then
          (if (Pawn|IsLocallyControlled _playerref)
            _))
        (:else))
      (elif (Variables|Default|GetTP?)
        (Class|PrimitiveComponent|SetOwnerNoSee (Variables|Default|GetLaserBeam) true)
        (bind _asbp_weapon_base_2 (Utilities|Casting|CastToBP_WeaponBase (Components|GetOwner))
          (:then
            (Variables|/Game/MultiplayerFPS/Game/Blueprints/Core/BP_WeaponBase.BP_WeaponBase_C|GetPlayerRef _asbp_weapon_base_2
              (:then
                _)
              (:else
                (Variables|Default|SetTP true :!label _label))))
          (:CastFailed
            (goto _label)))
        (Class|PrimitiveComponent|SetCastHiddenShadow (Variables|Default|GetStaticMesh) true)))))

(event EventBeginPlay
  (|CallParentFunction)
  (CallFunction|MCVisibility))

(event EventTick
  (params (DeltaSeconds :type Float%20%28single-precision%29))
  (|CallParentFunction DeltaSeconds)
  (if (not (Variables|Default|GetTP))
    (CallFunction|Linetrace)))

(event EventUpdateVisibility
  (params (NewViewMode :type Boolean))
  ;[1 1 1] Toggle
  (if (Variables|Default|GetFP?)
    (Class|PrimitiveComponent|SetOwnerNoSee (Variables|Default|GetStaticMesh) NewViewMode)
    (else
      (Class|PrimitiveComponent|SetOwnerNoSee (Variables|Default|GetStaticMesh) (not NewViewMode)))))

(event Collision|EventActorBeginOverlap
  (params (OtherActor :type Actor%20Object%20Reference))
  (|CallParentFunction OtherActor) ; This node is disabled and will not be called.\nDrag off pins to build functionality.
)

(event EventToggleLaserFlashlight
  (params (Toggle :type Boolean))
  ;[1 1 1] Toggle
  (bind _output_get (Variables|Default|SetLaserFlashlightToggled Toggle))
  (if _output_get
    (Rendering|SetVisibility (Variables|Default|GetLaserDot) true false)
    (else
      (Rendering|SetVisibility (Variables|Default|GetLaserDot) false false))))

(event EventLaserEvent
  (params (Toggle :type Boolean))
  ;[1 1 1] Set IR material
  (bind _output_get (Variables|Default|SetInfrared Toggle))
  (if _output_get
    (Rendering|Material|SetMaterial (Variables|Default|GetLaserBeam) 0 "/Game/MultiplayerFPS/Game/Weapons/Attachments/Laser/Meshes/Materials/M_Infrared.M_Infrared")
    (else
      (Rendering|Material|SetMaterial (Variables|Default|GetLaserBeam) 0 "/Game/MultiplayerFPS/Game/Weapons/Attachments/Laser/Meshes/Materials/M_Infrared_Inst.M_Infrared_Inst"))))

(fn ConstructionScript
  (|CallParentFunction))

(fn Linetrace
  (bind _start (Variables|Default|GetStart))
  (bind _returnvalue (Transformation|GetWorldLocation _start))
  (if (Variables|Default|GetLaserFlashlightToggled)
    (bind _outhit (Collision|LineTraceByChannel _returnvalue (+ _returnvalue (* (Math|Vector|GetForwardVector (Transformation|GetWorldRotation _start)) 8e+03)) "TraceTypeQuery1" false (Utilities|Array|MakeArray (Components|GetOwner)) "None" true "(R=1.000000,G=0.000000,B=0.000000,A=1.000000)" "(R=0.000000,G=1.000000,B=0.000000,A=1.000000)" 0.01))
    (LocalVariables|SetBlockingHit (.bBlockingHit (Collision|BreakHitResult _outhit)))
    (LocalVariables|SetDistance (.Distance (Collision|BreakHitResult _outhit)))
    (LocalVariables|SetLocation (.Location (Collision|BreakHitResult _outhit)))
    (LocalVariables|SetNormal (.Normal (Collision|BreakHitResult _outhit)))
    (LocalVariables|SetTraceEnd (.TraceEnd (Collision|BreakHitResult _outhit)))
    (Rendering|SetVisibility (Variables|Default|GetLaserDot) (LocalVariables|GetBlockingHit) false)
    (if (LocalVariables|GetBlockingHit)
      (Variables|Default|SetHitLocation (LocalVariables|GetLocation))
      (if (Variables|Default|GetInfrared)
        (Transformation|SetWorldScale3D (Variables|Default|GetLaserBeam) (Math|Vector|MakeVector (/ (LocalVariables|GetDistance) 15.0) 6.0 6.0))
        (else
          (Transformation|SetWorldScale3D (Variables|Default|GetLaserBeam) (Math|Vector|MakeVector (/ (LocalVariables|GetDistance) 15.0) 1.0 1.0))))
      (if (not (Variables|Default|GetTP?))
        (Transformation|SetWorldLocation (Variables|Default|GetLaserDot) (Variables|Default|GetHitLocation) false false)
        (Transformation|SetWorldRotation (Variables|Default|GetLaserDot) (Math|Rotator|MakeRotfromX (LocalVariables|GetNormal)) false false))
      (else
        (Variables|Default|SetHitLocation (LocalVariables|GetTraceEnd))))))