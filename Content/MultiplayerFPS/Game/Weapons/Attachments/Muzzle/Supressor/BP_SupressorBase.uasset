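; Base Blueprint for a weapon suppressor muzzle attachment that handles first/third-person mesh visibility and heat visuals.
; On BeginPlay it runs a visibility event that makes the FP mesh owner-only and shadowless, and hides the TP mesh from the owner while keeping its hidden shadow.
; UpdateVisibility flips owner visibility on view-mode changes.
; HeatUp and Cooldown both write the supplied heat to the mesh materials' Temperature parameter.
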(event Custom|MC_Visibility
  ;[1 1 1] Set FP and TP parts Visiblity
  (if (Variables|Default|GetVisibility)
    (if (Variables|Default|GetFP?)
      (Rendering|SetOnlyOwnerSee (Variables|Default|GetStaticMesh) true :!class /Script/Engine.PrimitiveComponent)
      (Rendering|SetCastShadow (Variables|Default|GetStaticMesh) false)
      (elif (Variables|Default|GetTP?)
        (Class|PrimitiveComponent|SetOwnerNoSee (Variables|Default|GetStaticMesh) true)
        (Class|PrimitiveComponent|SetCastHiddenShadow (Variables|Default|GetStaticMesh) true)))))

(event EventBeginPlay
  (|CallParentFunction)
  (CallFunction|MCVisibility))

(event EventCooldown
  (params (HeatAmt :type Float%20%28double-precision%29))
  ;[1 1 1] Set Temperature Material
  (Rendering|Material|SetScalarParameterValueonMaterials (Variables|Default|GetStaticMesh) "Temperature" HeatAmt))

(event EventUpdateVisibility
  (params (NewViewMode :type Boolean))
  (if (Variables|Default|GetFP?)
    (Class|PrimitiveComponent|SetOwnerNoSee (Variables|Default|GetStaticMesh) NewViewMode)
    (else
      (Class|PrimitiveComponent|SetOwnerNoSee (Variables|Default|GetStaticMesh) (not NewViewMode)))))

(event EventHeatUp
  (params (HeatAmt :type Float%20%28double-precision%29))
  ;[1 1 1] Set Temperature Material
  (Rendering|Material|SetScalarParameterValueonMaterials (Variables|Default|GetStaticMesh) "Temperature" HeatAmt))

(fn ConstructionScript
  (|CallParentFunction))