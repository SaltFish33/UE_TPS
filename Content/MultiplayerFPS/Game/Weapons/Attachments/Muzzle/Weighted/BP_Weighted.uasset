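; Weighted muzzle attachment actor for weapons, whose static mesh is shown or hidden according to whether it is the first-person or third-person copy.
; On BeginPlay it calls MC_Visibility, which makes the FP mesh owner-only without shadows and hides the TP mesh from its owner while keeping a hidden shadow.
; UpdateVisibility toggles owner-no-see oppositely on the two copies when the view mode changes.
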(event Custom|MC_Visibility
  ;[1 1 1] Set FP and TP parts Visiblity
  (if (Variables|Default|GetVisibility)
    (if (Variables|Default|GetFP?)
      (Rendering|SetOnlyOwnerSee (Variables|Default|GetStaticMesh) true :!class /Script/Engine.PrimitiveComponent)
      (Rendering|SetCastShadow (Variables|Default|GetStaticMesh) false)
      (elif (Variables|Default|GetTP?)
        (Class|PrimitiveComponent|SetOwnerNoSee (Variables|Default|GetStaticMesh) true)
        (Class|PrimitiveComponent|SetCastHiddenShadow (Variables|Default|GetStaticMesh) true)))))

(event EventBeginPlay
  (|CallParentFunction)
  (CallFunction|MCVisibility))

(event EventTick
  (params (DeltaSeconds :type Float%20%28single-precision%29))
  (|CallParentFunction DeltaSeconds) ; This node is disabled and will not be called.\nDrag off pins to build functionality.
)

(event EventUpdateVisibility
  (params (NewViewMode :type Boolean))
  (if (Variables|Default|GetFP?)
    (Class|PrimitiveComponent|SetOwnerNoSee (Variables|Default|GetStaticMesh) NewViewMode)
    (else
      (Class|PrimitiveComponent|SetOwnerNoSee (Variables|Default|GetStaticMesh) (not NewViewMode)))))

(event Collision|EventActorBeginOverlap
  (params (OtherActor :type Actor%20Object%20Reference))
  (|CallParentFunction OtherActor) ; This node is disabled and will not be called.\nDrag off pins to build functionality.
)

(fn ConstructionScript
  (|CallParentFunction))