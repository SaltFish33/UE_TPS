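; Base picture-in-picture scope attachment that renders a scene capture onto a lens material for the first-person copy.
; BeginPlay creates a per-client render target and dynamic material at runtime and hides the owner's components from the capture.
; A roughly 60 Hz tick captures only while AllowRTCapture is set, intended for ADS only, though EnablePIP's assignment is unwired here.
; UpdateVisibility flips mesh owner visibility by view mode and FP flag.
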(event EventEnablePIP
  (params (Enabled :type Boolean))
  ;[1 1 1] Enable PIP
)

(event EventBeginPlay
  ;[1 1 1] Create RT
  (|CallParentFunction)
  (if (Variables|Default|GetFP?)
    (bind _output_get (Variables|Default|SetSceneCapture (Variables|Default|GetSceneCaptureComponent2D)))
    (bind _returnvalue (Rendering|CreateRenderTarget2D 256 256 "RTF_RGBA16f")) ; Must be created in run time so each client has their own RT, otherwise all clients see same RT
    (Variables|/Script/Engine.SceneCaptureComponent2D|SetTextureTarget (Variables|Default|GetSceneCaptureComponent2D) _returnvalue)
    (bind _returnvalue_2 (Rendering|Material|CreateDynamicMaterialInstance (Variables|Default|GetStaticMesh) (Variables|Default|GetPIPMaterialIndex) (Variables|Default|GetPIPMaterial) "None" :!class /Script/Engine.PrimitiveComponent))
    (bind _output_get_2 (Variables|Default|SetMat _returnvalue_2))
    (Rendering|Material|SetMaterial (Variables|Default|GetStaticMesh) (Variables|Default|GetPIPMaterialIndex) _output_get_2)
    (Rendering|Material|SetTextureParameterValue _output_get_2 "RenderTarget" (Variables|/Script/Engine.SceneCaptureComponent2D|GetTextureTarget _output_get))
    (Class|SceneCaptureComponent|HideActorComponents (Variables|Default|GetSceneCaptureComponent2D) (Components|GetOwner) true)))

(event EventTick
  (params (DeltaSeconds :type Float%20%28single-precision%29))
  (|CallParentFunction DeltaSeconds)
  (if (Variables|Default|GetFP?)
    (if (Variables|Default|GetAllowRTCapture)
      (Rendering|SceneCapture|CaptureScene (Variables|Default|GetSceneCaptureComponent2D) :!class /Script/Engine.SceneCaptureComponent2D))
    (else
      (Variables|Default|SetAllowRTCapture false))))

(event EventUpdateVisibility
  (params (NewViewMode :type Boolean))
  (if (Variables|Default|GetFP?)
    (Class|PrimitiveComponent|SetOwnerNoSee (Variables|Default|GetStaticMesh) NewViewMode)
    (else
      (Class|PrimitiveComponent|SetOwnerNoSee (Variables|Default|GetStaticMesh) (not NewViewMode)))))

(event Collision|EventActorBeginOverlap
  (params (OtherActor :type Actor%20Object%20Reference))
  (|CallParentFunction OtherActor) ; This node is disabled and will not be called.\nDrag off pins to build functionality.
)

(fn ConstructionScript
  (|CallParentFunction)
  (Actor|Tick|SetActorTickInterval 0.016))