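; Mounted thermal optic attachment, filed under 8X optics, that shows a picture-in-picture scope image.
; On BeginPlay, only when the FP flag is set, it creates a render target at runtime for its scene capture component.
; A dynamic instance of the thermal PIP reticle material on one static mesh material slot receives that render target as its texture.
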(event EventBeginPlay
  (|CallParentFunction)
  (if (Variables|Default|GetFP?)
    (bind _output_get (Variables|Default|SetSceneCaptureComponent2D (Variables|Default|GetSceneCaptureComponent2D)))
    (bind _returnvalue (Rendering|CreateRenderTarget2D 256 256 "RTF_RGBA16f"))
    (Variables|/Script/Engine.SceneCaptureComponent2D|SetTextureTarget (Variables|Default|GetSceneCaptureComponent2D) _returnvalue)
    (bind _returnvalue_2 (Rendering|Material|CreateDynamicMaterialInstance (Variables|Default|GetStaticMesh) 4 "/Game/MultiplayerFPS/Game/Weapons/Attachments/Optic/Thermal/Mesh/Materials/M_ThermalPIPReticle_Inst.M_ThermalPIPReticle_Inst" "None" :!class /Script/Engine.PrimitiveComponent))
    (bind _output_get_2 (Variables|Default|SetScope_DMI _returnvalue_2))
    (Rendering|Material|SetMaterial (Variables|Default|GetStaticMesh) 4 _output_get_2)
    (Rendering|Material|SetTextureParameterValue _output_get_2 "RenderTarget" (Variables|/Script/Engine.SceneCaptureComponent2D|GetTextureTarget _output_get))))

(event Collision|EventActorBeginOverlap
  (params (OtherActor :type Actor%20Object%20Reference))
  (|CallParentFunction OtherActor) ; This node is disabled and will not be called.\nDrag off pins to build functionality.
)

(event EventTick
  (params (DeltaSeconds :type Float%20%28single-precision%29))
  (|CallParentFunction DeltaSeconds) ; This node is disabled and will not be called.\nDrag off pins to build functionality.
)

(fn ConstructionScript
  (|CallParentFunction))