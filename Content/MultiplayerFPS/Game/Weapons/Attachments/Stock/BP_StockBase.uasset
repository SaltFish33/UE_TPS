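; BP_StockBase is the base Blueprint for weapon stock attachments in a multiplayer FPS, handling first-person and third-person mesh visibility.
; On BeginPlay it sets up the mesh: FP parts are owner-only without shadows, while TP parts hide from the owner but cast hidden shadows.
; UpdateVisibility flips owner-no-see from a view mode flag, inversely for FP and non-FP parts.
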(event Custom|MC_Visibility
  ;[1 1 1] Set FP and TP parts Visiblity
  (if (Variables|Default|GetVisibility)
    (if (Variables|Default|GetFP?)
      (Rendering|SetOnlyOwnerSee (Variables|Default|GetStaticMesh) true :!class /Script/Engine.PrimitiveComponent)
      (Rendering|SetCastShadow (Variables|Default|GetStaticMesh) false)
      (elif (Variables|Default|GetTP?)
        (Class|PrimitiveComponent|SetOwnerNoSee (Variables|Default|GetStaticMesh) true)
        (Class|PrimitiveComponent|SetCastHiddenShadow (Variables|Default|GetStaticMesh) true)))))

(event EventBeginPlay
  (|CallParentFunction)
  (CallFunction|MCVisibility))

(event EventUpdateVisibility
  (params (NewViewMode :type Boolean))
  (if (Variables|Default|GetFP?)
    (Class|PrimitiveComponent|SetOwnerNoSee (Variables|Default|GetStaticMesh) NewViewMode)
    (else
      (Class|PrimitiveComponent|SetOwnerNoSee (Variables|Default|GetStaticMesh) (not NewViewMode)))))

(fn ConstructionScript
  (|CallParentFunction))