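; BP_M4A1 is the M4A1 primary weapon Blueprint, a child that leaves BeginPlay and construction to its parent class.
; Its own logic is the ToggleMagazineVisibility event, which swaps material slot 3 on the first-person and third-person meshes.
; Hiding applies an invisible material to both at once, while showing restores the body material on the first-person mesh, then on the third-person mesh after a short delay.
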(event EventBeginPlay
  (|CallParentFunction))

(event Collision|EventActorBeginOverlap
  (params (OtherActor :type Actor%20Object%20Reference)))

(event EventTick
  (params (DeltaSeconds :type Float%20%28single-precision%29)))

(event EventToggleMagazineVisibility
  (params (Visibility :type Boolean))
  (if Visibility
    (Rendering|Material|SetMaterial (Variables|Default|GetFPMesh) 3 "/Game/MultiplayerFPS/Game/Weapons/Primary/M4A1/Mesh/Materials/M_M4a1_Body.M_M4a1_Body")
    (Utilities|FlowControl|Delay 0.1)
    (Rendering|Material|SetMaterial (Variables|Default|GetTPMesh) 3 "/Game/MultiplayerFPS/Game/Weapons/Primary/M4A1/Mesh/Materials/M_M4a1_Body.M_M4a1_Body")
    (else
      (Rendering|Material|SetMaterial (Variables|Default|GetFPMesh) 3 "/Game/MultiplayerFPS/Game/Effects/M_Invisible.M_Invisible"))))

(fn ConstructionScript
  (|CallParentFunction))