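; BP_AK74Light is an AK-74 primary weapon Blueprint for the multiplayer FPS, built on a parent weapon class.
; ToggleMagazineVisibility hides the magazine by swapping material slot 3 on the first- and third-person meshes to an invisible material.
; Showing it restores the body material on the first-person mesh immediately and on the third-person mesh after a short delay.
; The construction script and GetSightTransform only pass through to the parent.
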(event EventBeginPlay
  (|CallParentFunction) ; This node is disabled and will not be called.\nDrag off pins to build functionality.
)

(event Collision|EventActorBeginOverlap
  (params (OtherActor :type Actor%20Object%20Reference)))

(event EventTick
  (params (DeltaSeconds :type Float%20%28single-precision%29)))

(event EventToggleMagazineVisibility
  (params (Visibility :type Boolean))
  (if Visibility
    (Rendering|Material|SetMaterial (Variables|Default|GetFPMesh) 3 "/Game/MultiplayerFPS/Game/Weapons/Primary/AK-74/Mesh/Materials/Main/M_AK-74_Body.M_AK-74_Body")
    (Utilities|FlowControl|Delay 0.1)
    (Rendering|Material|SetMaterial (Variables|Default|GetTPMesh) 3 "/Game/MultiplayerFPS/Game/Weapons/Primary/AK-74/Mesh/Materials/Main/M_AK-74_Body.M_AK-74_Body")
    (else
      (Rendering|Material|SetMaterial (Variables|Default|GetFPMesh) 3 "/Game/MultiplayerFPS/Game/Effects/M_Invisible.M_Invisible"))))

(fn ConstructionScript
  (|CallParentFunction))

(fn GetSightTransform
  (bind (_relativesighttransform _camdistance) (|CallParentFunction))
  (return _relativesighttransform _camdistance))