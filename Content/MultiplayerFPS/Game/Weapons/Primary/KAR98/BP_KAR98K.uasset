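; KAR98K weapon Blueprint for the multiplayer FPS, extending its parent with control over magazine visibility.
; The ToggleMagazineVisibility event swaps material slot 1 on the first-person and third-person meshes between the rifle material and an invisible one instead of hiding components.
; Showing updates the third-person mesh after a short delay, while hiding updates both meshes at once.
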(event EventBeginPlay
  (|CallParentFunction))

(event Collision|EventActorBeginOverlap
  (params (OtherActor :type Actor%20Object%20Reference)))

(event EventTick
  (params (DeltaSeconds :type Float%20%28single-precision%29)))

(event EventToggleMagazineVisibility
  (params (Visibility :type Boolean))
  (if Visibility
    (Rendering|Material|SetMaterial (Variables|Default|GetFPMesh) 1 "/Game/MultiplayerFPS/Game/Weapons/Primary/KAR98/Mesh/Materials/M_KAR98K.M_KAR98K")
    (Utilities|FlowControl|Delay 0.1)
    (Rendering|Material|SetMaterial (Variables|Default|GetTPMesh) 1 "/Game/MultiplayerFPS/Game/Weapons/Primary/KAR98/Mesh/Materials/M_KAR98K.M_KAR98K")
    (else
      (Rendering|Material|SetMaterial (Variables|Default|GetFPMesh) 1 "/Game/MultiplayerFPS/Game/Effects/M_Invisible.M_Invisible"))))

(fn ConstructionScript
  (|CallParentFunction))